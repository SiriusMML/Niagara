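; BP_Launcher is an actor that fires a Niagara homing missile effect at a BP_Target in the level.
; On BeginPlay it enables player input, finds the target actor and passes its location and a projectile count to the Missiles system as user variables.
; Pressing F activates the system with a reset and prints a debug message.
; The target location is sampled once, so the effect does not follow later target movement.
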(event EventBeginPlay
  (Input|EnableInput (Game|GetPlayerController 0))
  (bind _returnvalue (Actor|GetActorOfClass "/Game/Niagara/HomingMissile/BP_Target.BP_Target_C"))
  (Variables|Default|SetTarget _returnvalue)
  (Niagara|SetNiagaraVariable(Vector3) (Variables|Default|GetMissiles) "TargetLocation" (Transformation|GetActorLocation (Variables|Default|GetTarget)))
  (Niagara|SetNiagaraVariable(Float) (Variables|Default|GetMissiles) "NumberOfProjectiles" 1e+02))

(event Input|KeyboardEvents|F
  (params (Key :type Key%20Structure :default "None"))
  (:Pressed
    (Components|Activation|Activate (Variables|Default|GetMissiles) true)
    (Development|PrintString "Hello")))

(fn ConstructionScript)